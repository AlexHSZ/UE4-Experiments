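; BP_Interactable is an interactable cube actor that changes colour while it has focus.
; On BeginPlay it creates a dynamic material instance on the Cube and caches its original Colour parameter as the default.
; StartFocus sets that parameter to FocusedColour, and EndFocus restores the cached default.
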(event EventBeginPlay
  ;[1 1 1] Storing Colour Details
  (bind _returnvalue (Rendering|Material|CreateDynamicMaterialInstance (Variables|Default|GetCube) 0 0 "None" :!class /Script/Engine.PrimitiveComponent))
  (bind _output_get (Variables|Default|SetMaterialInstance _returnvalue))
  (bind _returnvalue_2 (Rendering|Material|GetVectorParameterValue _output_get "Colour" :!class /Script/Engine.MaterialInstanceDynamic))
  (Variables|Default|SetDefault%20Colour _returnvalue_2))

(event EventStartFocus
  (Rendering|Material|SetVectorParameterValue (Variables|Default|GetMaterialInstance) "Colour" (Variables|Default|GetFocused%20Colour) :!class /Script/Engine.MaterialInstanceDynamic))

(event EventEndFocus
  (Rendering|Material|SetVectorParameterValue (Variables|Default|GetMaterialInstance) "Colour" (Variables|Default|GetDefault%20Colour) :!class /Script/Engine.MaterialInstanceDynamic))

(fn ConstructionScript)